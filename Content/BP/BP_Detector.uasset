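; BP_Detector is an actor that exercises the perception subsystem by switching detection on and off in a repeating cycle.
; After a short startup delay, BeginPlay starts detection with its DetectionForm and fixed area and time settings, then alternates stopping and restarting on timed delays.
; An ActorsDetected event prints detected actor names, but the node binding it to the subsystem's detection event is disconnected and never runs.
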(event `self.ReceiveBeginPlay`
  (bind _returnvalue (subsystem `PerceptionSubsystem`))
  (bind (_perceptioninfo_detectarea _perceptioninfo_detectiontime) (break `PerceptionInfo` (make `PerceptionInfo` 400.0 1.0)))
  (`KismetSystemLibrary.Delay` 0.2)
  (`PerceptionSubsystem.DoDetection` _returnvalue self (`self.Detection Form`) (make `PerceptionInfo` _perceptioninfo_detectarea _perceptioninfo_detectiontime) :!label _label)
  (`KismetSystemLibrary.Delay` 4.0)
  (`PerceptionSubsystem.StopDetecting` _returnvalue self)
  (`KismetSystemLibrary.Delay` 4.0)
  (goto _label))

(event `Actors Detected`
  (params (DetectedActor :type "Actor Object Reference"))
  (`KismetSystemLibrary.PrintString` (`KismetSystemLibrary.GetDisplayName` DetectedActor)))

(fn `UserConstructionScript`)